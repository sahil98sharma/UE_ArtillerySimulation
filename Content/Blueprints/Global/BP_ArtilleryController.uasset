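; BP_ArtilleryController is a player controller that switches the player between the artillery Gunner and Observer pawns.
; On BeginPlay it adds the input mapping context and caches references to both pawns found in the level.
; The IA_TogglePlayerControl action, gated by a settable CanToggleArtilleryControl flag, possesses the other pawn and updates the CurrentController enum.
; Print strings report reference setup and control changes.
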(event `self.ReceiveBeginPlay`
  (`self.SetupInputSystemRef`)
  (`self.SetPawnRefs`))

(event `EnhancedInput|/Game/Input/Actions/IA_TogglePlayerControl`
  (params (ActionValue :type Boolean) (ElapsedSeconds :type "Float (double-precision)") (TriggeredSeconds :type "Float (double-precision)") (InputAction :type "InputAction Object Reference" :default "/Game/Input/Actions/IA_TogglePlayerControl.IA_TogglePlayerControl"))
  (:`Triggered`
    (if (`self.bCanToggleArtilleryControl`)
      (`self.ToggleArtilleryControl`))))

(fn `SetCurrentController`
  (params (newController :type "/Game/Blueprints/Enums/EArtilleryController Enum" :default "NewEnumerator0"))
  (bind _output_get (set `self.CurrentController` newController))
  (`KismetSystemLibrary.PrintString` (`KismetStringLibrary.Concat_StrStr` "Current Controller Set to: " (`|GetEnumeratorNameAsString` _output_get))))

(fn `SetPawnRefs`
  (`|ExecutionSequence`
    (:`then_0`
      (bind _returnvalue (`GameplayStatics.GetActorOfClass` "/Game/Blueprints/Pawns/BP_GunnerPawn.BP_GunnerPawn_C"))
      (`/Engine/EditorBlueprintResources/StandardMacros.IsValid` _returnvalue
        (:`Is Valid`
          (set `self.Gunner` _returnvalue)
          (`KismetSystemLibrary.PrintString` "BP_Gunner Ref Set"))))
    (:`then_1`
      (bind _returnvalue_2 (`GameplayStatics.GetActorOfClass` "/Game/Blueprints/Pawns/BP_ObserverPawn.BP_ObserverPawn_C"))
      (`/Engine/EditorBlueprintResources/StandardMacros.IsValid` _returnvalue_2
        (:`Is Valid`
          (set `self.Observer` _returnvalue_2)
          (`KismetSystemLibrary.PrintString` "BP_ObserverPawn Ref Set"))))))

(fn `SetToggleArtilleryControl`
  (params (bCanToggleArtilleryControl :type Boolean))
  (set `self.bCanToggleArtilleryControl` bCanToggleArtilleryControl))

(fn `SetupInputSystemRef`
  (`EnhancedInputSubsystemInterface.AddMappingContext` (pcsubsystem `EnhancedInputLocalPlayerSubsystem` self) "/Game/Input/NewInputMappingContext.NewInputMappingContext" 0 (struct)))

(fn `ToggleArtilleryControl`
  (switch `/Game/Blueprints/Enums/EArtilleryController` (`self.CurrentController`)
    (:`NewEnumerator0`
      (`self.Possess` (`self.Gunner`))
      (`self.SetCurrentController` "NewEnumerator1"))
    (:`NewEnumerator1`
      (`self.Possess` (`self.Observer`))
      (`self.SetCurrentController` "NewEnumerator0"))))

(fn `UserConstructionScript`)