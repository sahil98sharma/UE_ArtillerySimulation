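; Actor component that places a target marker in the world where the player's mouse cursor points.
; TargetTrace deprojects player 0's cursor and line traces along that direction up to Range on the Camera channel, with timed debug drawing enabled.
; On a hit, it moves the existing CurrentTargetMarker to the hit location, or spawns and stores a BP_TargetMarker if none is valid.
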(event `Event TargetTrace`
  (bind (_worldlocation _worlddirection) (`PlayerController.DeprojectMousePositionToWorld` (`GameplayStatics.GetPlayerController` 0)))
  (bind (_outhit _returnvalue) (`KismetSystemLibrary.LineTraceSingle` :`Start` _worldlocation :`End` (+ _worldlocation (* _worlddirection (`self.Range`))) :`TraceChannel` "TraceTypeQuery2" :`DrawDebugType` "ForDuration" :`DrawTime` 2.0))
  (if _returnvalue
    (`/Engine/EditorBlueprintResources/StandardMacros.IsValid` (`self.CurrentTargetMarker`)
      (:`Is Valid`
        (bind (_bblockinghit _binitialoverlap _time _distance _location) (`GameplayStatics.BreakHitResult` _outhit))
        (`Actor.K2_SetActorLocation` (`self.CurrentTargetMarker`) _location false false))
      (:`Is Not Valid`
        (bind _returnvalue_2 (`|SpawnActorFromClass` "/Game/Blueprints/Actors/BP_TargetMarker.BP_TargetMarker_C" (`KismetMathLibrary.Conv_VectorToTransform` _location) "Undefined" "MultiplyWithRoot" null null))
        (set `self.CurrentTargetMarker` _returnvalue_2)))))